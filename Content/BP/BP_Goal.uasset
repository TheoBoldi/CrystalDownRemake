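; BP_Goal is a damageable objective with an outer goal mesh around a crystal, each with its own collider.
; GetDamage subtracts from CurrentHealth, set to MaxHealth at construction, and advances an enum state at quarter-health thresholds, at most one step per hit.
; At zero health it hides the goal and makes the crystal collidable.
; The next hit hides the crystal and only prints "EndRound"; event graph nodes are disabled.
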(fn `GetDamage`
  (params (Damage :type Integer))
  (bind _output_get (set `self.CurrentHealth` (- (`self.CurrentHealth`) Damage)))
  (`KismetSystemLibrary.PrintString` (`KismetStringLibrary.Conv_IntToString` _output_get))
  (if (`|EnumEquality` (`self.State`) "NewEnumerator0")
    (if (<= (`self.CurrentHealth`) (/ (* (`self.MaxHealth`) 3) 4))
      (bind _output_get_2 (set `self.State` "NewEnumerator1"))
      (`KismetSystemLibrary.PrintString` (`|GetEnumeratorNameAsString` _output_get_2)))
    (elif (`|EnumEquality` (`self.State`) "NewEnumerator1")
      (if (<= (`self.CurrentHealth`) (/ (* (`self.MaxHealth`) 2) 4))
        (bind _output_get_3 (set `self.State` "NewEnumerator2"))
        (`KismetSystemLibrary.PrintString` (`|GetEnumeratorNameAsString` _output_get_3)))
      (elif (`|EnumEquality` (`self.State`) "NewEnumerator2")
        (if (<= (`self.CurrentHealth`) (/ (* (`self.MaxHealth`) 1) 4))
          (bind _output_get_4 (set `self.State` "NewEnumerator3"))
          (`KismetSystemLibrary.PrintString` (`|GetEnumeratorNameAsString` _output_get_4)))
        (elif (`|EnumEquality` (`self.State`) "NewEnumerator3")
          (if (<= (`self.CurrentHealth`) 0)
            (`PrimitiveComponent.SetCollisionProfileName` (`self.MainCollider`) "NoCollision" true)
            (`SceneComponent.SetVisibility` (`self.GoalMesh`) false false)
            (`PrimitiveComponent.SetCollisionProfileName` (`self.CrystalCollider`) "BlockAll" true)
            (bind _output_get_5 (set `self.State` "NewEnumerator4"))
            (`KismetSystemLibrary.PrintString` (`|GetEnumeratorNameAsString` _output_get_5)))
          (elif (`|EnumEquality` (`self.State`) "NewEnumerator4")
            (`PrimitiveComponent.SetCollisionProfileName` (`self.CrystalCollider`) "NoCollision" true)
            (`SceneComponent.SetVisibility` (`self.CrystalMesh`) false false)
            (`KismetSystemLibrary.PrintString` "EndRound")))))))

(fn `UserConstructionScript`
  (set `self.CurrentHealth` (`self.MaxHealth`)))