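; Destructible blue statue that breaks through four successive stages each time a BP_Ball hits its collision component.
; A hit counter selects the stage event, which creates a dynamic material instance on that stage's statue mesh.
; A timeline drives "Display Frame" from 1 to 180, playing a baked rigid-body vertex animation texture (VAT) destruction.
; The final stage also disables the statue's collision.
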(event `State1`
  (bind _returnvalue (`PrimitiveComponent.CreateDynamicMaterialInstance` (`self.SM_Statue_State_1_2`) 0 null "None"))
  (bind (_direction _newtrack_0) (`Timeline|PlayAnim` :!via `PlayFromStart`)
    (:`Update`
      (`MaterialInstanceDynamic.SetScalarParameterValue` _returnvalue "Display Frame" (`KismetMathLibrary.Lerp` 1.0 180.0 _newtrack_0)))))

(event `State2`
  (bind _returnvalue (`PrimitiveComponent.CreateDynamicMaterialInstance` (`self.SM_Statue_State_2_3`) 0 "/Game/Import/Statue/MI_RBD_VAT_Statue_State_2.MI_RBD_VAT_Statue_State_2" "None"))
  (bind (_direction _newtrack_0) (`Timeline|Timeline` :!via `PlayFromStart`)
    (:`Update`
      (`MaterialInstanceDynamic.SetScalarParameterValue` _returnvalue "Display Frame" (`KismetMathLibrary.Lerp` 1.0 180.0 _newtrack_0)))))

(event `State3`
  (bind _returnvalue (`PrimitiveComponent.CreateDynamicMaterialInstance` (`self.SM_Statue_State_3_4`) 0 "/Game/Import/Statue/MI_RBD_VAT_Statue_State_3.MI_RBD_VAT_Statue_State_3" "None"))
  (bind (_direction _newtrack_0) (`Timeline|Timeline_0` :!via `PlayFromStart`)
    (:`Update`
      (`MaterialInstanceDynamic.SetScalarParameterValue` _returnvalue "Display Frame" (`KismetMathLibrary.Lerp` 1.0 180.0 _newtrack_0)))))

(event `State_4`
  (`PrimitiveComponent.SetCollisionEnabled` (`self.COL_Statue`) "NoCollision")
  (bind _returnvalue (`PrimitiveComponent.CreateDynamicMaterialInstance` (`self.SM_Statue_State_4_5`) 0 "/Game/Import/Statue/MI_RBD_VAT_Statue_State_4.MI_RBD_VAT_Statue_State_4" "None"))
  (bind (_direction _newtrack_0) (`Timeline|Timeline_1` :!via `PlayFromStart`)
    (:`Update`
      (`MaterialInstanceDynamic.SetScalarParameterValue` _returnvalue "Display Frame" (`KismetMathLibrary.Lerp` 1.0 180.0 _newtrack_0)))))

(event `self.COL_Statue.OnComponentHit`
  (params (HitComponent :type "PrimitiveComponent Object Reference") (OtherActor :type "Actor Object Reference") (OtherComp :type "PrimitiveComponent Object Reference") (NormalImpulse :type "Vector Structure") (Hit :type "HitResult Structure (by ref)"))
  (cast `/Game/BP/BP_Ball` OtherActor)
  (set `self.State` (+ (`self.State`) 1))
  (switch `int` (`self.State`)
    (:`1`
      (`self.State1`))
    (:`2`
      (`self.State2`))
    (:`3`
      (`self.State3`))
    (:`4`
      (`self.State_4`))))

(fn `UserConstructionScript`)