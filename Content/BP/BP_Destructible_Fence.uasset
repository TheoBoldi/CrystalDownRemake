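; Destructible fence actor that breaks in two stages when hit by BP_Ball.
; Each ball hit on the collision component increments a state counter, triggering the first stage, then the second, which also disables fence collision.
; Each stage creates a dynamic material on its own mesh, and a timeline drives its "Display Frame" parameter, playing baked frame animation through the material instead of simulating physics.
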(event `State1`
  (bind _returnvalue (`PrimitiveComponent.CreateDynamicMaterialInstance` (`self.SM_Fence_Stage_1`) 0 null "None"))
  (bind (_direction _newtrack_0) (`Timeline|PlayAnim` :!via `PlayFromStart`)
    (:`Update`
      (`MaterialInstanceDynamic.SetScalarParameterValue` _returnvalue "Display Frame" (`KismetMathLibrary.Lerp` 1.0 300.0 _newtrack_0)))))

(event `State2`
  (`PrimitiveComponent.SetCollisionEnabled` (`self.COL_Fence`) "NoCollision")
  (bind _returnvalue (`PrimitiveComponent.CreateDynamicMaterialInstance` (`self.SM_Fence_Stage_2`) 0 null "None"))
  (bind (_direction _newtrack_0) (`Timeline|Timeline` :!via `PlayFromStart`)
    (:`Update`
      (`MaterialInstanceDynamic.SetScalarParameterValue` _returnvalue "Display Frame" (`KismetMathLibrary.Lerp` 1.0 300.0 _newtrack_0)))))

(event `self.COL_Fence.OnComponentHit`
  (params (HitComponent :type "PrimitiveComponent Object Reference") (OtherActor :type "Actor Object Reference") (OtherComp :type "PrimitiveComponent Object Reference") (NormalImpulse :type "Vector Structure") (Hit :type "HitResult Structure (by ref)"))
  (cast `/Game/BP/BP_Ball` OtherActor)
  (set `self.State` (+ (`self.State`) 1))
  (switch `int` (`self.State`)
    (:`1`
      (`self.State1`))
    (:`2`
      (`self.State2`))))

(fn `UserConstructionScript`)