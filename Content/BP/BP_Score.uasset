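; BP_Score keeps Red and Blue team scores and restarts the round each time a point is awarded.
; AddPointToTeam increments one score based on the destroyed crystal's team and prints it as debug text.
; It then respawns every BP_character and resets all BP_Destructible_Fence and BP_Goal actors through class-wide actor searches.
; It also looks up ScoreWidget instances but leaves the result unused.
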(fn `AddPointToTeam`
  (params (CrystalDestroyedTeam :type "/Game/BP/TeamsEnum Enum" :default "NewEnumerator0"))
  (if (`|EnumEquality` CrystalDestroyedTeam "NewEnumerator0")
    (bind _output_get (set `self.RedTeamScore` (+ (`self.RedTeamScore`) 1)))
    (`KismetSystemLibrary.PrintString` "Red Team Score : ")
    (`KismetSystemLibrary.PrintString` (`KismetStringLibrary.Conv_IntToString` _output_get))
    (else
      (bind _output_get_2 (set `self.BlueTeamScore` (+ (`self.BlueTeamScore`) 1)))
      (`KismetSystemLibrary.PrintString` "Blue Team Score : ")
      (`KismetSystemLibrary.PrintString` (`KismetStringLibrary.Conv_IntToString` _output_get_2))))
  (`WidgetBlueprintLibrary.GetAllWidgetsOfClass` "/Game/BP/Widgets/ScoreWidget.ScoreWidget_C")
  (bind _outactors (`GameplayStatics.GetAllActorsOfClass` "/Game/BP/BP_character.BP_character_C"))
  (for _array_element _outactors
    (`/Game/BP/BP_character.Respawn` _array_element))
  (bind _outactors_2 (`GameplayStatics.GetAllActorsOfClass` "/Game/BP/BP_Destructible_Fence.BP_Destructible_Fence_C"))
  (for _array_element_2 _outactors_2
    (`/Game/BP/BP_Destructible_Fence.ResetFence` _array_element_2))
  (bind _outactors_3 (`GameplayStatics.GetAllActorsOfClass` "/Game/BP/BP_Goal.BP_Goal_C"))
  (for _array_element_3 _outactors_3
    (`/Game/BP/BP_Goal.ResetGoal` _array_element_3)))

(fn `UserConstructionScript`)